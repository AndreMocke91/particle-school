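; Ice beam effect actor that stretches a particle beam from its own location toward a Target actor.
; Each tick, and on construction, it passes the target location to the Beam component and line-traces toward it on the Visibility channel.
; On a hit, it moves BeamHit to the impact point aligned to the surface normal and updates the beam's distance, midpoint offset and orientation, all measured to the Target rather than the impact.
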(event `self.ReceiveTick`
  (params (DeltaSeconds :type "Float (single-precision)"))
  (`self.SetParticleEffectTargets`))

(fn `SetParticleEffectTargets`
  (bind _beamhit (`self.BeamHit`))
  (bind _returnvalue (`self.K2_GetActorLocation` (`self.Target`)))
  (bind _returnvalue_2 (- (`self.K2_GetActorLocation`) (`self.K2_GetActorLocation` (`self.Target`))))
  (`/Engine/EditorBlueprintResources/StandardMacros.IsValid` (`self.Target`)
    (:`Is Valid`
      (`NiagaraComponent.SetVariableVec3` (`self.Beam`) "TargetVector" _returnvalue)
      (bind (_outhit _returnvalue_3) (`KismetSystemLibrary.LineTraceSingle` (`self.K2_GetActorLocation`) _returnvalue "TraceTypeQuery1"))
      (if _returnvalue_3
        (bind (_bblockinghit _binitialoverlap _time _distance _location _impactpoint _normal) (`GameplayStatics.BreakHitResult` _outhit))
        (`SceneComponent.K2_SetWorldLocation` _beamhit _impactpoint false false)
        (`SceneComponent.K2_SetWorldRotation` _beamhit (`KismetMathLibrary.MakeRotationFromAxes` _normal) false false)
        (`NiagaraComponent.SetVariableFloat` (`self.Beam`) "DistanceToTarget" (`self.GetDistanceTo` (`self.Target`)))
        (`NiagaraComponent.SetVariableVec3` (`self.Beam`) "Offset" (/ _returnvalue_2 (-2.0 -2.0 -2.0)))
        (`NiagaraComponent.SetVariableVec3` (`self.Beam`) "OrientationVector" (* (`KismetMathLibrary.Normal` _returnvalue_2) (1.0 1.0 1.0)))))))

(fn `UserConstructionScript`
  (`self.SetParticleEffectTargets`))